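; Enemy actor that flies in a straight line and ends the game when it overlaps the player.
; On BeginPlay a random roll against TraceRate either aims and rotates it at the player's current position or keeps its forward vector, and Tick moves it along that fixed direction.
; Overlap destroys both actors, spawns an explosion and shows the game-over widget.
; It also holds an Escape key FlipFlop that toggles the pause menu.
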(event `self.ReceiveBeginPlay`
  (if (<= (`KismetMathLibrary.RandomFloatInRange` 0.0 1.0) (`self.TraceRate`))
    (bind _returnvalue (`GameplayStatics.GetActorOfClass` "/Game/BluePrints/BP_Player.BP_Player_C"))
    (`/Engine/EditorBlueprintResources/StandardMacros.IsValid` _returnvalue
      (:`Is Valid`
        (bind _output_get (set `self.Direction` (`KismetMathLibrary.Normal` (- (`self.K2_GetActorLocation` _returnvalue) (`self.K2_GetActorLocation`)))))
        ;[1 1 1] Enemy 회전
        (`self.K2_SetActorRotation` (`KismetMathLibrary.MakeRotFromXZ` _output_get (`self.GetActorUpVector`)))))
    (else
      (set `self.Direction` (`self.GetActorForwardVector`)))))

(event `self.ReceiveTick`
  (params (DeltaSeconds :type "Float (single-precision)"))
  (`self.K2_SetActorLocation` (+ (`self.K2_GetActorLocation`) (* (* (`self.Direction`) (`self.MoveSpeed`)) DeltaSeconds))))

(event `self.ReceiveActorBeginOverlap`
  (params (OtherActor :type "Actor Object Reference"))
  ;[1 1 1] 플레이어 충돌시 사망
  (bind _asbp_player (cast `/Game/BluePrints/BP_Player` OtherActor))
  (`self.K2_DestroyActor` _asbp_player)
  (`GameplayStatics.SpawnEmitterAtLocation` "/Game/StarterContent/Particles/P_Explosion.P_Explosion" (`self.K2_GetActorLocation`))
  (`self.K2_DestroyActor`)
  ;[1 1 1] 게임오버
  (bind _returnvalue (`|CreateWidget` "/Game/UI/BP_GameOver.BP_GameOver_C"))
  (`UserWidget.AddToViewport` _returnvalue 0)
  (set `PlayerController.bShowMouseCursor` true (`GameplayStatics.GetPlayerController` 0)))

(event `Key|Escape`
  (params (Key :type "Key Structure"))
  (:`Pressed`
    (`/Engine/EditorBlueprintResources/StandardMacros.FlipFlop`
      (:`A`
        (bind _returnvalue (`|CreateWidget` "/Game/UI/BP_Pause.BP_Pause_C"))
        (`UserWidget.AddToViewport` _returnvalue 0)
        (set `PlayerController.bShowMouseCursor` true (`GameplayStatics.GetPlayerController` 0))
        (`GameplayStatics.SetGamePaused` true))
      (:`B`
        (`Widget.RemoveFromParent` _returnvalue)
        (`GameplayStatics.SetGamePaused` false)))))

(fn `UserConstructionScript`
  (locals (`Player ref` :type "Controller Object Reference")))